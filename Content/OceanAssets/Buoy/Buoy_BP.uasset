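; Ocean buoy actor with a point light that blinks at slightly irregular intervals.
; Tick feeds a Delay of randomized length of roughly a second, then flips LightOn and applies it to the light's visibility.
; The construction script applies the initial LightOn value to the light.
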(event `self.ReceiveTick`
  (params (DeltaSeconds :type "Float (single-precision)"))
  (bind _lighton (`self.LightOn`))
  (`parent.ReceiveTick` DeltaSeconds)
  (`KismetSystemLibrary.Delay` (`KismetMathLibrary.RandomFloatInRange` 1.0 1.5))
  (if _lighton
    (set `self.LightOn` false)
    (else
      (set `self.LightOn` true)))
  (`SceneComponent.SetVisibility` (`self.PointLight`) _lighton false))

(fn `UserConstructionScript`
  (`parent.UserConstructionScript`)
  (`SceneComponent.SetVisibility` (`self.PointLight`) (`self.LightOn`) false))